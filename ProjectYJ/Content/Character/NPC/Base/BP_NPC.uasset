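; Base NPC Blueprint that wanders randomly around the level on the navmesh.
; On BeginPlay it picks a random reachable point within a fixed radius of its current location and uses AI MoveTo to walk there.
; The move event calls itself again after a pause on success, or almost immediately on failure, forming an endless roaming loop.
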(event `self.ReceiveBeginPlay`
  (`self.MoveNPC`))

(event `MoveNPC`
  (bind _output_get (set `self.Random Location` (`NavigationSystemV1.K2_GetRandomReachablePointInRadius` (`self.K2_GetActorLocation`) 1000.0 null null)))
  (`|AIMoveTo` self _output_get null
    (:`OnSuccess`
      (`KismetSystemLibrary.Delay` 2.0)
      (`self.MoveNPC`))
    (:`OnFail`
      (`KismetSystemLibrary.Delay` 0.1)
      (`self.MoveNPC`))))

(fn `UserConstructionScript`)